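; Base buildable ammo crate that periodically resupplies living teammates inside its aura sphere once built.
; A looping server timer runs AmmoAuraEffect, where AmmoEffect adds missing clips or tops up partial ones, drawing on a finite or infinite supply.
; Sphere overlaps toggle teammates' HUD resupply icon, while build events set the mesh by remaining ammo.
; The older use-to-resupply path with per-player cooldowns is disconnected.
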(event OnComponentBeginOverlap(AreaOfEffectCollisionSphere)
  (params (OverlappedComponent :type Primitive%20Component%20Object%20Reference) (OtherActor :type Actor%20Object%20Reference) (OtherComp :type Primitive%20Component%20Object%20Reference) (OtherBodyIndex :type Integer) (bFromSweep :type Boolean) (SweepResult :type Hit%20Result%20Structure%20%28by%20ref%29))
  (Utilities|IsValid OtherActor
    (:Is%20Valid
      (bind _asdfbase_character (Utilities|Casting|CastToDFBaseCharacter OtherActor))
      (CallFunction|SetIconVisibility _asdfbase_character true))))

(event OnComponentEndOverlap(AreaOfEffectCollisionSphere)
  (params (OverlappedComponent :type Primitive%20Component%20Object%20Reference) (OtherActor :type Actor%20Object%20Reference) (OtherComp :type Primitive%20Component%20Object%20Reference) (OtherBodyIndex :type Integer))
  (Utilities|IsValid OtherActor
    (:Is%20Valid
      (bind _asdfbase_character (Utilities|Casting|CastToDFBaseCharacter OtherActor))
      (CallFunction|SetIconVisibility _asdfbase_character false))))

(event Custom|Multicast%20Resupply
  ;[1 1 1] Unused code for interacting with ammo crate to get resupplied
)

(event Custom|Event%20Do%20Aura%20Effect
  (Networking|SwitchHasAuthority
    (:Authority
      (CallFunction|AmmoAuraEffect))))

(event Custom|Event%20On%20Aura%20Effect%20Begin
  (CallFunction|SetIconVisibilityOverlappingPawns true))

(event Custom|Event%20On%20Aura%20Effect%20End
  (CallFunction|SetIconVisibilityOverlappingPawns false))

(event EventTick
  (params (DeltaSeconds :type Float%20%28single-precision%29))
  (|CallParentFunction DeltaSeconds)
  (if (Variables|Default|GetbBuilt)
    (if (not (Variables|DONOTEDIT|GetbIsTimerSet))
      (Variables|DONOTEDIT|SetbIsTimerSet true)
      (CallFunction|EventonAuraEffectBegin)
      (Networking|SwitchHasAuthority
        (:Authority
          (bind _returnvalue (Utilities|Time|SetTimerbyEvent (delegate Custom|Event%20Do%20Aura%20Effect) (Variables|AmmoCrate|GetAuraEffectTimerInterval) true))
          (Variables|AmmoCrate|SetAuraEffectTimerHandle _returnvalue))))
    (elif (Variables|DONOTEDIT|GetbIsTimerSet)
      (Variables|DONOTEDIT|SetbIsTimerSet false)
      (CallFunction|EventonAuraEffectEnd)
      (Networking|SwitchHasAuthority
        (:Authority
          (Utilities|Time|ClearandInvalidateTimerbyHandle (Variables|AmmoCrate|GetAuraEffectTimerHandle)))))))

(event EventUsed
  (params (Invoker :type Actor%20Object%20Reference))
  ;[1 1 1] Unused code for interacting with ammo crate to get resupplied
)

(event EventHandleRepBuilt
  (CallFunction|SetMeshtoAmmoCount))

(event EventHandleHealthChangeBuildLevel
  (params (Old%20Health :type Float%20%28single-precision%29) (New%20Health :type Float%20%28single-precision%29) (Build%20Status :type Integer))
  (|CallParentFunction Old%20Health New%20Health Build%20Status)
  (CallFunction|SetMeshtoAmmoCount))

(fn ConstructionScript
  (|CallParentFunction)
  (Components|Sphere|SetSphereRadius (Variables|Default|GetAreaOfEffectCollisionSphere) (Variables|AmmoCrate|GetAuraRadius) true))

(fn SetMeshtoAmmoCount
  (Networking|CanExecuteCosmeticEvents
    (:True
      (if (Variables|Default|GetbBuilt)
        ;[1 1 1] Checks if less than 90% if so it goes to the next check
        (if (<= (Variables|AmmoCrate|GetAmmoRestoreRemaining) (Math|Float|Truncate (* (Variables|AmmoCrate|GetAmmoRestoreMax) 0.9)))
          ;[1 1 1] Setting to (Top) 2/3 ammo, (Bottom) or full ammo
          (Components|StaticMesh|SetStaticMesh (Variables|Default|GetStaticMesh) (Utilities|Array|Get(acopy) (Variables|Default|GetBuildStages) 2))
          (if (<= (Variables|AmmoCrate|GetAmmoRestoreRemaining) (Math|Float|Truncate (* (Variables|AmmoCrate|GetAmmoRestoreMax) 0.6)))
            (Components|StaticMesh|SetStaticMesh (Variables|Default|GetStaticMesh) (Utilities|Array|Get(acopy) (Variables|Default|GetBuildStages) 1))
            (if (== (Variables|AmmoCrate|GetAmmoRestoreRemaining) 0)
              (Components|StaticMesh|SetStaticMesh (Variables|Default|GetStaticMesh) (Utilities|Array|Get(acopy) (Variables|Default|GetBuildStages)))))
          (else
            (Components|StaticMesh|SetStaticMesh (Variables|Default|GetStaticMesh) (Utilities|Array|Get(acopy) (Variables|Default|GetBuildStages) 3))))))))

(fn AmmoEffect
  (params (Pawn :type DF%20Base%20Character%20Object%20Reference) (Ammo :type Integer))
  (bind _inventory (Variables|/Script/DonkehFramework.DFBaseCharacter|GetInventory Pawn))
  (bind _items (Variables|/Script/DonkehFramework.DFInventoryComponent|GetItems _inventory))
  (Utilities|IsValid Pawn
    (:Is%20Valid
      (for _array_element _items
        (Utilities|IsValid _array_element
          (:Is%20Valid
            (bind _ashdbase_weapon (Utilities|Casting|CastToHDBaseWeapon _array_element))
            (if (Math|Boolean|ANDBoolean (!= _ashdbase_weapon self) (<= (Variables|/Script/HDMain.HDBaseWeapon|GetAmmoReplenishmentDelay _ashdbase_weapon) 0.0) (> (Utilities|Set|Length (Variables|/Script/DonkehFramework.DFBaseGun|GetSupportedAmmoClips _ashdbase_weapon)) 0)) ; Check if the pawn should receive\nmore ammo for this weapon
              (if (> (- (Variables|/Script/DonkehFramework.DFBaseGun|GetStartingAmmoClips _ashdbase_weapon) (Class|DFBaseGun|GetNumFreeAmmoClips _ashdbase_weapon false true)) 0) ; Issue fresh ammo clip or refill pre-existing (partial) ones?
                (bind _result (Utilities|Set|ToArray (Variables|/Script/DonkehFramework.DFBaseGun|GetSupportedAmmoClips _ashdbase_weapon)))
                (bind _returnvalue (Class|DFBaseAmmoClip|StoreAmmoinInventory _inventory (* (.StartingClipAmmo (Utilities|GetClassDefaults (Utilities|Array|Get(acopy) _result))) (Math|Integer|Min(Integer) (- (Variables|/Script/DonkehFramework.DFBaseGun|GetStartingAmmoClips _ashdbase_weapon) (Class|DFBaseGun|GetNumFreeAmmoClips _ashdbase_weapon false true)) Ammo)) (Utilities|Array|Get(acopy) _result)))
                (Class|DFBlueprintFunctions|PrintStringtoLog (Utilities|String|Append (Utilities|String|ToString(Integer) _returnvalue) " Ammo Clips dispensed to Pawn Inventory") "VeryVerbose")
                (Math|Integer|IncrementInt (LocalVariables|GetNumberOfClipsRestored) :!label _label)
                (elif (not (Variables|AmmoCrate|GetbDoNotRefillPartialClips))
                  (LocalVariables|SetNumPartialClipsFilled 0)
                  (bind _array_element_2 (Utilities|Array|ForEachLoopwithBreak _items :!label _label_2)
                    (:LoopBody
                      (bind _asdfbase_ammo_clip (Utilities|Casting|CastToDFBaseAmmoClip _array_element_2))
                      (if (and (< (Variables|/Script/DonkehFramework.DFBaseAmmoClip|GetCurrentClipAmmo _asdfbase_ammo_clip) (Variables|/Script/DonkehFramework.DFBaseAmmoClip|GetMaxClipAmmo _asdfbase_ammo_clip)) (Utilities|Set|Contains (Variables|/Script/DonkehFramework.DFBaseGun|GetSupportedAmmoClips _ashdbase_weapon) (Utilities|GetClass _asdfbase_ammo_clip)))
                        (bind _gunowner (Variables|/Script/DonkehFramework.DFBaseAmmoClip|GetGunOwner _asdfbase_ammo_clip)
                          (:then)
                          (:else
                            (Class|DFBaseAmmoClip|StoreAmmo _asdfbase_ammo_clip (- (Variables|/Script/DonkehFramework.DFBaseAmmoClip|GetMaxClipAmmo _asdfbase_ammo_clip) (Variables|/Script/DonkehFramework.DFBaseAmmoClip|GetCurrentClipAmmo _asdfbase_ammo_clip)))
                            (Utilities|FlowControl|Sequence
                              (:then_0
                                (goto _label))
                              (:then_1
                                (bind _result_2 (Math|Integer|IncrementInt (LocalVariables|GetNumPartialClipsFilled))
                                  (:%20%20
                                    (if (>= _result_2 Ammo)
                                      (goto _label_2 Break)))))))))))))))))
      (Development|PrintString (Utilities|String|ToString(Integer) (Variables|AmmoCrate|GetAmmoRestoreRemaining)))
      (return (LocalVariables|GetNumberOfClipsRestored)))))

(fn GetCooldownforPlayer
  (params (Actor :type Actor%20Object%20Reference))
  (bind _outactors (Actor|GetAllActorsOfClass "/HDAssets/Items/Equipment/Utility/Construction/Cooldowns/BP_Ammo_Cooldown_Manager_Base.BP_Ammo_Cooldown_Manager_Base_C"))
  (bind _array_element (Utilities|Array|ForEachLoopwithBreak _outactors :!label _label)
    (:LoopBody
      ;[1 1 1] Checks if there is a cooldown manager of the same owner
      (if (== (Game|GetInstigatorController Actor) (Components|GetOwner _array_element))
        (LocalVariables|SetTheCooldown _array_element)
        (LocalVariables|SetbFound true)
        (goto _label Break)))
    (:Completed
      ;[1 1 1] Spawns a new one
      (if (LocalVariables|GetbFound)
        (return (LocalVariables|GetTheCooldown))
        (else
          (Networking|SwitchHasAuthority
            (:Authority
              (bind _returnvalue (Game|SpawnActorfromClass "/HDAssets/Items/Equipment/Utility/Construction/Cooldowns/BP_Ammo_Cooldown_Manager_Base.BP_Ammo_Cooldown_Manager_Base_C" (Math|Transform|MakeTransform "0, 0, 0") "Undefined" (Game|GetInstigatorController Actor) 0))
              (return _returnvalue))))))))

(fn DisplayAmmoCooldown
  (params (Actor :type Actor%20Object%20Reference) (Cooldown%20Seconds :type Integer))
  (bind _returnvalue (Math|Conversions|ToFloat(Integer) Cooldown%20Seconds))
  (bind (_remainder _returnvalue_2) (Math|Float|Division(WholeandRemainder) _returnvalue 6e+01))
  (bind _returnvalue_3 (Math|Float|Truncate _remainder))
  (bind _returnvalue_4 (Utilities|String|ToString(Integer) _returnvalue_3))
  (if (> Cooldown%20Seconds 0)
    (bind _ashdplayer_controller (Utilities|Casting|CastToHDPlayerController (Game|GetInstigatorController Actor))
      (:then
        (bind _ashdhud (Utilities|Casting|CastToHDHUD (HUD|GetHUD _ashdplayer_controller))
          (:then
            (bind _asbp_hdhudbase (Utilities|Casting|CastToBP_HDHUDBase _ashdhud)
              (:then
                (if (== _returnvalue_2 0)
                  (Default|AddBasicNotification _asbp_hdhudbase (Utilities|Struct|MakeFUINotificationInfo false 0 "NewEnumerator0" true (Utilities|Text|ToText(String) (Utilities|String|Append "<Normal>Ammo crate is on cooldown! Cooldown elapses in: " _returnvalue_4 " seconds </>")) "<Bold>{timer}</>" 5.0))
                  (else
                    (Default|AddBasicNotification _asbp_hdhudbase (Utilities|Struct|MakeFUINotificationInfo false 0 "NewEnumerator0" true (Utilities|Text|ToText(String) (Utilities|String|Append "<Normal>Ammo crate is on cooldown! Cooldown elapses in: " (Utilities|String|ToString(Integer) _returnvalue_2) ":" _returnvalue_4 "</>")) "<Bold>{timer}</>" 5.0)))))
              (:CastFailed
                (Development|PrintString "Failed BP Cast for HUD" true true "(R=1.000000,G=0.000000,B=0.000000,A=1.000000)"))))
          (:CastFailed
            (Development|PrintString "Failed C++ Cast for Hud" true true "(R=1.000000,G=0.000000,B=0.000000,A=1.000000)"))))
      (:CastFailed
        (Development|PrintString "Cast to Controller Failed" true true "(R=1.000000,G=0.000000,B=0.000000,A=1.000000)")))
    (else
      (bind _ashdplayer_controller_2 (Utilities|Casting|CastToHDPlayerController (Game|GetInstigatorController Actor))
        (:then
          (bind _ashdhud_2 (Utilities|Casting|CastToHDHUD (HUD|GetHUD _ashdplayer_controller_2))
            (:then
              (bind _asbp_hdhudbase_2 (Utilities|Casting|CastToBP_HDHUDBase _ashdhud_2)
                (:then
                  (Default|AddBasicNotification _asbp_hdhudbase_2 (Utilities|Struct|MakeFUINotificationInfo false 0 "NewEnumerator0" true (Utilities|Text|ToText(String) "<Normal>Resupplied Successfully</>") "<Bold>{timer}</>" 5.0)))
                (:CastFailed
                  (Development|PrintString "Failed BP Cast for HUD" true true "(R=1.000000,G=0.000000,B=0.010000,A=1.000000)"))))
            (:CastFailed
              (Development|PrintString "Failed C++ Cast for Hud" true true "(R=1.000000,G=0.000000,B=0.000000,A=1.000000)"))))
        (:CastFailed
          (Development|PrintString "Cast to Controller Failed" true true "(R=1.000000,G=0.000000,B=0.000000,A=1.000000)"))))))

(fn SetIconVisibilityOverlappingPawns
  (params (bVisibility :type Boolean))
  (for _array_element (Collision|GetOverlappingActors (Variables|Default|GetAreaOfEffectCollisionSphere) "/Script/DonkehFramework.DFBaseCharacter" :!class /Script/Engine.PrimitiveComponent) ; Get all players currently within our aura
    (Utilities|IsValid _array_element
      (:Is%20Valid
        (bind _asdfbase_character (Utilities|Casting|CastToDFBaseCharacter _array_element))
        (CallFunction|SetIconVisibility _asdfbase_character bVisibility)))))

(fn SetIconVisibility
  (params (Pawn :type DF%20Base%20Character%20Object%20Reference) (bVisiblity :type Boolean))
  (if (and (Class|DFBaseCharacter|IsAlive Pawn) (== (Variables|/Script/DonkehFramework.DFBaseCharacter|GetTeamNum Pawn) (Variables|Default|GetOwningTeam))) ; Check if the player is on our team
    (bind _ashdplayer_controller (Utilities|Casting|CastToHDPlayerController (Pawn|GetController Pawn)))
    (bind _asbp_hdhudbase (Utilities|Casting|CastToBP_HDHUDBase (HUD|GetHUD _ashdplayer_controller)))
    ;[0 1 1] Update visibility of "Ammo Resupply" Player Effect HUD icon
    (Default|SetAmmoResupplyEffectVisibility _asbp_hdhudbase bVisiblity)))

(fn AmmoAuraEffect
  (Utilities|FlowControl|Sequence
    (:then_0
      (Utilities|Array|Clear (Variables|DONOTEDIT|GetAffectedPawns))
      (for _array_element (Collision|GetOverlappingActors (Variables|Default|GetAreaOfEffectCollisionSphere) "/Script/DonkehFramework.DFBaseCharacter" :!class /Script/Engine.PrimitiveComponent) ; Get all players currently within our aura
        (Utilities|IsValid _array_element
          (:Is%20Valid
            (bind _asdfbase_character (Utilities|Casting|CastToDFBaseCharacter _array_element))
            (Utilities|Array|Add (Variables|DONOTEDIT|GetAffectedPawns) _asdfbase_character)))))
    (:then_1
      (for _array_element_2 (Variables|DONOTEDIT|GetAffectedPawns)
        (Utilities|IsValid _array_element_2
          (:Is%20Valid
            (bind _output_get (LocalVariables|SetCurrentPawn _array_element_2))
            (if (and (Class|DFBaseCharacter|IsAlive _output_get) (== (Variables|/Script/DonkehFramework.DFBaseCharacter|GetTeamNum _output_get) (Variables|Default|GetOwningTeam))) ; Check if the player should be restored
              (if (Variables|AmmoCrate|GetbInfiniteRestore)
                (CallFunction|AmmoEffect (LocalVariables|GetCurrentPawn) (Variables|AmmoCrate|GetAmmoClipRestoreAmount))
                (elif (< (Variables|AmmoCrate|GetAmmoClipRestoreAmount) (Variables|AmmoCrate|GetAmmoRestoreRemaining)) ; How much ammo do we have remaining
                  (bind _clipsrestored (CallFunction|AmmoEffect (LocalVariables|GetCurrentPawn) (Variables|AmmoCrate|GetAmmoClipRestoreAmount)))
                  (Variables|AmmoCrate|SetAmmoRestoreRemaining (- (Variables|AmmoCrate|GetAmmoRestoreRemaining) _clipsrestored))
                  (elif (> (Variables|AmmoCrate|GetAmmoRestoreRemaining) 0)
                    (CallFunction|AmmoEffect (LocalVariables|GetCurrentPawn) (Variables|AmmoCrate|GetAmmoRestoreRemaining))
                    (Variables|AmmoCrate|SetAmmoRestoreRemaining 0)
                    (else
                      (return))))))))))))