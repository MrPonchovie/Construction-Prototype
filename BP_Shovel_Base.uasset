(event Custom|Event%20Set%20Range%20Increment%20Server
  (params (In%20Increment :type Integer))
  ;[1 1 1] Changing Degree Increment
  (Variables|Default|SetRange%20Increment In%20Increment))

(event Custom|Event%20Set%20Degree%20Increment%20Server
  (params (In%20Increment :type Integer))
  ;[1 1 1] Changing Degree Increment
  (Variables|Default|SetDegree%20Increment In%20Increment))

(event Custom|Cycle%20Build%20Mode
  ;[1 1 1] Changing Degree Increment
  (|CallParentFunction)
  (Utilities|FlowControl|Delay 0.2)
  (bind _out_increment (CallFunction|ReadComponentTags))
  (CallFunction|EventSetDegreeIncrementServer _out_increment)
  (bind _range_increment (CallFunction|ConvertDegreeInctoRangeInc _out_increment))
  (CallFunction|EventSetRangeIncrementServer _range_increment)
  (Default|SetDegreeIncrement (Variables|Default|GetWidget) _out_increment))

(event Custom|Show%20Initial%20Notification
  (bind _returnvalue (Class|InputSettings|GetInputSettings))
  (bind _returnvalue_2 (Class|InputSettings|GetInputSettings))
  (bind _outmappings (Class|InputSettings|GetActionMappingbyName _returnvalue_2 "Aim"))
  (bind _outmappings_2 (Class|InputSettings|GetActionMappingbyName _returnvalue "AimToggle"))
  (bind _output (Utilities|Array|Get(acopy) _outmappings_2))
  (bind _output_2 (Utilities|Array|Get(acopy) _outmappings))
  (bind _returnvalue_3 (Class|KismetInputLibrary|KeyGetDisplayName (.key _output)))
  (bind _returnvalue_4 (Class|KismetInputLibrary|KeyGetDisplayName (.key _output_2)))
  (bind _returnvalue_5 (Utilities|String|ToString(Text) _returnvalue_4))
  (bind _returnvalue_6 (Utilities|String|ToString(Text) _returnvalue_3))
  (bind _returnvalue_7 (Utilities|Enum|Equal(Enum) _returnvalue_6 "None"))
  (if (Utilities|Enum|Equal(Enum) _returnvalue_5 "None")
    (if _returnvalue_7
      (Default|AddBasicNotification (Variables|Default|GetNotification%20Widget) (Utilities|Struct|MakeFUINotificationInfo false 0 "NewEnumerator0" true "<Normal>Please bind the \"AimToggle\" or \"Aim\" keybinds to use this item properly</>" "" 1e+01))
      (else
        ;[1 1 1] AimToggle Keybind Active
        (Default|AddBasicNotification (Variables|Default|GetNotification%20Widget) (Utilities|Struct|MakeFUINotificationInfo false 0 "NewEnumerator0" true (Utilities|Text|ToText(String) (Utilities|String|Append "<Normal>Use \"" _returnvalue_6 "\" to change between building and destroying</>")) "" 1e+01))))
    (elif _returnvalue_7
      ;[1 1 1] AimToggle Keybind Active
      (Default|AddBasicNotification (Variables|Default|GetNotification%20Widget) (Utilities|Struct|MakeFUINotificationInfo false 0 "NewEnumerator0" true (Utilities|Text|ToText(String) (Utilities|String|Append "<Normal>Use \"" _returnvalue_5 "\" to change between building and destroying</>")) "" 1e+01))
      (else
        ;[1 1 1] Both Keybinds Active
        (Default|AddBasicNotification (Variables|Default|GetNotification%20Widget) (Utilities|Struct|MakeFUINotificationInfo false 0 "NewEnumerator0" true (Utilities|Text|ToText(String) (Utilities|String|Append "<Normal>Use \"" _returnvalue_5 "\" or \"" _returnvalue_6 "\" to change between building and destroying</>")) "" 1e+01))))))

(event EventFire
  (CallFunction|Linetrace))

(event EventOnEquip
  (params (LastItem :type DF%20Base%20Item%20Object%20Reference))
  (bind _pawnowner (Variables|Default|GetPawnOwner))
  (bind _playerstate (Variables|/Script/Engine.Pawn|GetPlayerState _pawnowner))
  (bind _ownerc (CallFunction|GetControllerfromPlayerState _playerstate))
  (|CallParentFunction LastItem)
  (Networking|CanExecuteCosmeticEvents
    (:True
      (bind _foundwidgets (Widget|GetAllWidgetsOfClass "/HDAssets/Items/Equipment/Utility/Construction/WBP_Shovel_UI.WBP_Shovel_UI_C" true))
      (for _array_element _foundwidgets
        (if (== (Widget|GetOwningPlayer _array_element) _ownerc)
          (Widget|RemovefromParent _array_element)))
      (bind _asbp_hdplayer_controller (Utilities|Casting|CastToBP_HDPlayerController _ownerc)
        (:then
          (CallFunction|GetValidNotificationWidget _asbp_hdplayer_controller)
          (CallFunction|ShowInitialNotification)
          (bind _returnvalue (UserInterface|CreateWidget "/HDAssets/Items/Equipment/Utility/Construction/WBP_Shovel_UI.WBP_Shovel_UI_C" _asbp_hdplayer_controller))
          (bind _output_get (Variables|Default|SetWidget _returnvalue))
          (UserInterface|Viewport|AddtoPlayerScreen _output_get 1)
          (Default|SetDegreeIncrement (Variables|Default|GetWidget) (Variables|Default|GetDegree%20Increment))
          (Default|SetRangeIncrement (Variables|Default|GetWidget) (Variables|Default|GetRange%20Increment)))
        (:CastFailed
          (Development|PrintString "NOT A REAL PLAYER"))))))

(event EventOnUnEquip
  (params (bPlayAnimAndWait :type Boolean) (bLeavingPawnInventory :type Boolean))
  (|CallParentFunction bPlayAnimAndWait bLeavingPawnInventory)
  (Networking|CanExecuteCosmeticEvents
    (:True
      (Widget|RemovefromParent (Variables|Default|GetWidget)))))

(fn ConstructionScript
  (bind _building (Variables|Default|GetBuilding))
  (|CallParentFunction)
  (Variables|Default|SetSights (Utilities|Array|MakeArray _building (Variables|Default|GetUnBuild)))
  (Variables|Default|SetCurrentSight _building))

(fn ReadComponentTags
  (bind _currentsight (Variables|Default|GetCurrentSight))
  (bind _componenttags (Variables|/Script/Engine.ActorComponent|GetComponentTags _currentsight))
  (bind _output (Utilities|Array|Get(acopy) _componenttags))
  (bind _returnvalue (Utilities|String|ToString(Name) _output))
  (bind _returnvalue_2 (Math|Conversions|ToInteger(Byte) _returnvalue))
  (bind _output_get (Variables|Default|SetDegree%20Increment _returnvalue_2))
  (Development|PrintString (Utilities|String|ToString(Integer) _returnvalue_2) true true "(R=1.000000,G=0.000000,B=0.915568,A=1.000000)")
  (return _output_get))

(fn Linetrace
  (Utilities|IsValid (Variables|Default|GetPlayer) :!label _label
    (:Is%20Valid
      (bind (_outhit _returnvalue) (Collision|LineTraceByChannel (Transformation|GetWorldLocation (Class|DFBasePlayerCharacter|GetCamera1P (Variables|Default|GetPlayer))) (+ (Transformation|GetWorldLocation (Class|DFBasePlayerCharacter|GetCamera1P (Variables|Default|GetPlayer))) (* (Math|Vector|GetForwardVector (Class|DFBasePlayerCharacter|GetCamera1P (Variables|Default|GetPlayer))) (Variables|Default|GetTrace%20DistanceCM))) "TraceTypeQuery3" false (Utilities|Array|MakeArray (Class|DFBaseItem|GetPawnOwner) self) "ForDuration"))
      (if _returnvalue
        (Development|PrintString (Class|KismetSystemLibrary|GetPathName (.HitActor (Collision|BreakHitResult _outhit))))
        (if (Actor|ActorHasTag (.HitActor (Collision|BreakHitResult _outhit)) "Buildable_Object")
          (bind _asbp_hd_buildable_world_base (Utilities|Casting|CastToBP_HD_Buildable_World_Base (.HitActor (Collision|BreakHitResult _outhit)))
            (:then
              (bind _new_health (Default|FuncUpdateHealth _asbp_hd_buildable_world_base 34.0 (Variables|Default|GetDegree%20Increment) (Class|DFBlueprintFunctions|GetTeamNum (Variables|Default|GetPlayer))))
              (Networking|CanExecuteCosmeticEvents
                (:True
                  (Default|UpdateConstructionTooltip (Variables|Default|GetWidget) (Variables|/HDAssets/Items/Equipment/Utility/Construction/BP_HD_Buildable_World_Base.BP_HD_Buildable_World_Base_C|GetUIName _asbp_hd_buildable_world_base) (/ _new_health (Variables|/HDAssets/Items/Equipment/Utility/Construction/BP_HD_Buildable_World_Base.BP_HD_Buildable_World_Base_C|GetMaximumHealth _asbp_hd_buildable_world_base)))
                  (Audio|PlaySoundatLocation "/HDCore/Marketplace/BulletEffectsPack/BulletHitVFX_SFX/ESounds/Cue/SFX_Bullet_Impact_Sandbag.SFX_Bullet_Impact_Sandbag" (.Location (Collision|BreakHitResult _outhit)) "0, 0, 0" 0.8 1.0 0.0 0 0 (Components|GetOwner)))))
            (:CastFailed
              (Class|DFBlueprintFunctions|PrintTexttoLog "Cast to DSFP_Buildable_Object failed despite filters" "Error" true)))
          (else
            (Development|PrintString "Object doesn't have Buildable tag, ignoring." true true "(R=1.000000,G=0.879168,B=0.000000,A=1.000000)")))
        (else
          (Class|DFBlueprintFunctions|PrintTexttoLog "Caught nothing in shovel line trace. (NOTE: This is NOT an error)" "Warning"))))
    (:Is%20Not%20Valid
      (bind _ashdplayer_character (Utilities|Casting|CastToHDPlayerCharacter (Class|DFBaseItem|GetPawnOwner))
        (:then
          (Variables|Default|SetPlayer _ashdplayer_character)
          (goto _label))
        (:CastFailed
          (Class|DFBlueprintFunctions|PrintTexttoLog "Failed to cast to C++ Controller" "Error" true))))))

(fn ConvertDegreeInctoRangeInc
  (params (Degree%20Increment :type Integer))
  (switch int Degree%20Increment
    (:Default
      _)
    (:1
      (bind _output_get (Variables|Default|SetRange%20Increment 1))
      (return _output_get))
    (:2
      _)
    (:3
      _)
    (:4
      _)
    (:5
      (bind _output_get_2 (Variables|Default|SetRange%20Increment 2))
      (return _output_get_2))
    (:6
      _)
    (:7
      _)
    (:8
      _)
    (:9
      _)
    (:10
      (bind _output_get_3 (Variables|Default|SetRange%20Increment 4))
      (return _output_get_3)))
  (Development|PrintString "Invalid Range Increment!" true true "(R=1.000000,G=0.000000,B=0.000000,A=1.000000)"))

(fn GetValidNotificationWidget
  (params (Target :type Player%20Controller%20Object%20Reference))
  (bind _ashdhud (Utilities|Casting|CastToHDHUD (HUD|GetHUD Target))
    (:then
      (bind _asbp_hdhudbase (Utilities|Casting|CastToBP_HDHUDBase _ashdhud)
        (:then
          (Variables|Default|SetNotification%20Widget _asbp_hdhudbase))
        (:CastFailed
          (Development|PrintString "Failed BP Cast for HUD" true true "(R=1.000000,G=0.000000,B=0.101476,A=1.000000)"))))
    (:CastFailed
      (Development|PrintString "Failed C++ Cast for Hud" true true "(R=1.000000,G=0.000000,B=0.000000,A=1.000000)"))))

(fn GenericNotification
  (params (Info%20Text :type Text))
  (Default|AddBasicNotification (Variables|Default|GetNotification%20Widget) (Utilities|Struct|MakeFUINotificationInfo false 0 "NewEnumerator0" true Info%20Text "" 5.0)))