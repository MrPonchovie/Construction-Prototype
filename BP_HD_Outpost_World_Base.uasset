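; Base outpost actor that owns nearby team buildables, limits their numbers and tracks whether it can be spawned at.
; Each tick, sphere overlaps set CanBeSpawnedAt from enemy players in overrun range and gather buildables in build range.
; Valid same-team buildables have decay halted and are tallied by type for QueryBuildCounts to check against maximums.
; On destruction, it starts decay on its buildables and releases them.
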(event EventTick
  (params (DeltaSeconds :type Float%20%28single-precision%29))
  (Utilities|FlowControl|Sequence
    (:then_0
      (Variables|Default|SetOwningOutpost 0)
      (bind _outactors (Collision|SphereOverlapActors (Transformation|GetActorLocation) (Variables|Outpost|GetOverrunRadiusCM) (Utilities|Array|MakeArray "ObjectTypeQuery3") "/HDAssets/Core/BP_HDPlayerCharacter.BP_HDPlayerCharacter_C" (Utilities|Array|MakeArray self)))
      (CallFunction|EvalCanbeSpawnedat _outactors)
      (bind _outactors_2 (Collision|SphereOverlapActors (Transformation|GetActorLocation) (Variables|Outpost|GetBuildRangeRadiusCM) (Utilities|Array|MakeArray "ObjectTypeQuery6") "/HDAssets/Items/Equipment/Utility/Construction/BP_HD_Buildable_World_Base.BP_HD_Buildable_World_Base_C" (Utilities|Array|MakeArray self)))
      (for _array_element _outactors_2
        (bind _asbp_hd_buildable_world_base (Utilities|Casting|CastToBP_HD_Buildable_World_Base _array_element))
        (Utilities|Array|AddUnique (Variables|DONOTEDIT|GetInfluences) _asbp_hd_buildable_world_base))
      (CallFunction|CheckActorsinInfluence)
      (for _array_element_2 (Variables|DONOTEDIT|GetInfluences)
        (Variables|/HDAssets/Items/Equipment/Utility/Construction/BP_HD_Buildable_World_Base.BP_HD_Buildable_World_Base_C|SetOwningOutpost _array_element_2 self)))
    (:then_1
      (Utilities|FlowControl|Delay 1.5)
      (|CallParentFunction DeltaSeconds))))

(event EventHandleDestroy
  (Actor|Tick|SetActorTickEnabled false)
  (for _array_element (Variables|DONOTEDIT|GetInfluences)
    (Default|EventBeginDecay _array_element true)
    (Variables|/HDAssets/Items/Equipment/Utility/Construction/BP_HD_Buildable_World_Base.BP_HD_Buildable_World_Base_C|SetOwningOutpost _array_element 0))
  (Actor|SetLifeSpan 0.1))

(fn ConstructionScript
  (|CallParentFunction)
  (Components|Sphere|SetSphereRadius (Variables|Default|GetBuildRangeSphere) (Variables|Outpost|GetBuildRangeRadiusCM) true)
  (Components|Sphere|SetSphereRadius (Variables|Default|GetOverrunSphere) (Variables|Outpost|GetOverrunRadiusCM) true))

(fn CheckActorsinInfluence
  (LocalVariables|SetTempVariables (Utilities|Struct|MakeFOutpostConstructionAmounts))
  (for _array_element (Variables|DONOTEDIT|GetInfluences)
    (Utilities|IsValid _array_element
      (:Is%20Valid
        (if (Math|Boolean|ANDBoolean (== (Variables|Default|GetOwningTeam) (Variables|/HDAssets/Items/Equipment/Utility/Construction/BP_HD_Buildable_World_Base.BP_HD_Buildable_World_Base_C|GetOwningTeam _array_element)) (Math|Boolean|NotEqual(Boolean) (Actor|ActorHasTag _array_element "HD_IgnoreRadio") true) (or (== (Variables|/HDAssets/Items/Equipment/Utility/Construction/BP_HD_Buildable_World_Base.BP_HD_Buildable_World_Base_C|GetOwningOutpost _array_element) self) (== (Variables|/HDAssets/Items/Equipment/Utility/Construction/BP_HD_Buildable_World_Base.BP_HD_Buildable_World_Base_C|GetOwningOutpost _array_element) 0)))
          (Variables|/HDAssets/Items/Equipment/Utility/Construction/BP_HD_Buildable_World_Base.BP_HD_Buildable_World_Base_C|SetOwningOutpost _array_element self)
          (Default|EventHaltDecay _array_element)
          (switch string (Variables|/HDAssets/Items/Equipment/Utility/Construction/BP_HD_Buildable_World_Base.BP_HD_Buildable_World_Base_C|GetUIName _array_element)
            (:Default
              (Development|PrintString (Utilities|String|Append "Unhandled Exception: " (Variables|/HDAssets/Items/Equipment/Utility/Construction/BP_HD_Buildable_World_Base.BP_HD_Buildable_World_Base_C|GetUIName _array_element)) true true "(R=1.000000,G=0.035135,B=0.000000,A=1.000000)" 5.0))
            (:SANDBAG%20WALL
              (LocalVariables|SetTempVariables (Utilities|Struct|MakeFOutpostConstructionAmounts (+ (.sandbagwalls (LocalVariables|GetTempVariables)) 1) (.ammocrates (LocalVariables|GetTempVariables)) (.doublehescowalls (LocalVariables|GetTempVariables)) (.sandbagroofs (LocalVariables|GetTempVariables)) (.ladders (LocalVariables|GetTempVariables)))))
            (:AMMO%20CRATE
              (LocalVariables|SetTempVariables (Utilities|Struct|MakeFOutpostConstructionAmounts (.sandbagwalls (LocalVariables|GetTempVariables)) (+ (.ammocrates (LocalVariables|GetTempVariables)) 1) (.doublehescowalls (LocalVariables|GetTempVariables)) (.sandbagroofs (LocalVariables|GetTempVariables)) (.ladders (LocalVariables|GetTempVariables)))))
            (:HESCO%20DOUBLE%20WALL
              (LocalVariables|SetTempVariables (Utilities|Struct|MakeFOutpostConstructionAmounts (.sandbagwalls (LocalVariables|GetTempVariables)) (.ammocrates (LocalVariables|GetTempVariables)) (+ (.doublehescowalls (LocalVariables|GetTempVariables)) 1) (.sandbagroofs (LocalVariables|GetTempVariables)) (.ladders (LocalVariables|GetTempVariables)))))
            (:SANDBAG%20ROOF
              (LocalVariables|SetTempVariables (Utilities|Struct|MakeFOutpostConstructionAmounts (.sandbagwalls (LocalVariables|GetTempVariables)) (.ammocrates (LocalVariables|GetTempVariables)) (.doublehescowalls (LocalVariables|GetTempVariables)) (+ (.sandbagroofs (LocalVariables|GetTempVariables)) 1) (.ladders (LocalVariables|GetTempVariables)))))
            (:LADDER
              (LocalVariables|SetTempVariables (Utilities|Struct|MakeFOutpostConstructionAmounts (.sandbagwalls (LocalVariables|GetTempVariables)) (.ammocrates (LocalVariables|GetTempVariables)) (.doublehescowalls (LocalVariables|GetTempVariables)) (.sandbagroofs (LocalVariables|GetTempVariables)) (+ (.ladders (LocalVariables|GetTempVariables)) 1)))))
          (else
            (Utilities|Array|AddUnique (LocalVariables|GetInvalidActors) _array_element :!label _label))))
      (:Is%20Not%20Valid
        (goto _label))))
  (for _array_element_2 (LocalVariables|GetInvalidActors)
    (Utilities|Array|RemoveItem (Variables|DONOTEDIT|GetInfluences) _array_element_2))
  (Variables|DONOTEDIT|SetCurrentBuildableAmount (LocalVariables|GetTempVariables))
  (return))

(fn QueryBuildCounts
  (params (QueryType :type Integer))
  (switch int QueryType
    (:Default
      (return true))
    (:0
      (if (> (+ (.sandbagwalls (Variables|DONOTEDIT|GetCurrentBuildableAmount)) 1) (.sandbagwalls (Variables|Outpost|GetMaximumBuildableAmount)))
        (return false)
        (else
          (return true))))
    (:1
      (if (> (+ (.ammocrates (Variables|DONOTEDIT|GetCurrentBuildableAmount)) 1) (.ammocrates (Variables|Outpost|GetMaximumBuildableAmount)))
        (return false)
        (else
          (return true))))
    (:2
      (if (> (+ (.doublehescowalls (Variables|DONOTEDIT|GetCurrentBuildableAmount)) 1) (.doublehescowalls (Variables|Outpost|GetMaximumBuildableAmount)))
        (return false)
        (else
          (return true))))
    (:3
      (if (> (+ (.sandbagroofs (Variables|DONOTEDIT|GetCurrentBuildableAmount)) 1) (.sandbagroofs (Variables|Outpost|GetMaximumBuildableAmount)))
        (return false)
        (else
          (return true))))
    (:4
      (if (> (+ (.ladders (Variables|DONOTEDIT|GetCurrentBuildableAmount)) 1) (.ladders (Variables|Outpost|GetMaximumBuildableAmount)))
        (return false)
        (else
          (return true))))))

(fn EvalCanbeSpawnedat
  (params (Array :type Array%20of%20Actor%20Object%20References))
  (bind _owningteam (Variables|Default|GetOwningTeam))
  (bind _array_element (Utilities|Array|ForEachLoopwithBreak Array :!label _label)
    (:LoopBody
      (bind _ashdplayer_character (Utilities|Casting|CastToHDPlayerCharacter _array_element))
      (if (not (Math|Boolean|ORBoolean (== (Variables|/Script/DonkehFramework.DFBaseCharacter|GetTeamNum _ashdplayer_character) _owningteam) (== _owningteam 255) (== (Variables|/Script/DonkehFramework.DFBaseCharacter|GetTeamNum _ashdplayer_character) 255)))
        (LocalVariables|SetResult (+ (LocalVariables|GetResult) 1))
        (goto _label Break)))
    (:Completed
      (Variables|Outpost|SetCanBeSpawnedAt (>= (LocalVariables|GetResult) (Variables|Outpost|GetOverrunAmount))))))

(fn OnRepCanbeSpawnedat)