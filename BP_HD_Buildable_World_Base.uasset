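; Base buildable world structure with team ownership, replicated health driving staged mesh swaps for construction and dig-down, and destruction at zero.
; Damage and build changes pass through FuncUpdateHealth, which scales dig-down differently for enemy teams.
; Structures needing a floor box-trace support points on BeginPlay and each authority Tick.
; Losing support triggers OnRep-driven, unstoppable decay on a looping server timer, and a despawn lifespan also applies.
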(event Custom|Event%20SetupOwnership
  (params (Owning%20Team :type Byte) (Owning%20Squad :type HD%20Squad%20State%20Object%20Reference))
  (Networking|SwitchHasAuthority
    (:Authority
      (Variables|DONOTEDIT|SetOwningTeam Owning%20Team)
      (Variables|DONOTEDIT|SetOwningSquad Owning%20Squad))))

(event Custom|Handle%20Destroy
  (Actor|SetLifeSpan 0.1))

(event Custom|Handle%20Rep%20Built)

(event Custom|Event%20Begin%20Decay
  (params (Can%20Stop :type Boolean))
  (Networking|SwitchHasAuthority
    (:Authority
      (if (not (Variables|DONOTEDIT|GetbDecaying))
        (Variables|DONOTEDIT|SetbDecaying true)
        (bind _returnvalue (Utilities|Time|SetTimerbyFunctionName 0 "FuncDecayTick" (Variables|Gameplay|GetDecayTickSpeed) true))
        (Variables|DONOTEDIT|SetDecayTimer _returnvalue)
        (Variables|DONOTEDIT|SetbCanStopDecay Can%20Stop)
        (Development|PrintString (Utilities|String|Append (Utilities|GetObjectName self) " is now decaying"))))))

(event Custom|Event%20Halt%20Decay
  (if (and (Variables|DONOTEDIT|GetbCanStopDecay) (Utilities|Time|IsValidTimerHandle (Variables|DONOTEDIT|GetDecayTimer)))
    (Variables|DONOTEDIT|SetbDecaying false)
    (Utilities|Time|PauseTimerbyHandle (Variables|DONOTEDIT|GetDecayTimer))
    (Development|PrintString (Utilities|String|Append (Utilities|GetObjectName self) " is no longer decaying"))))

(event EventBeginPlay
  (if (not (Variables|DONOTEDIT|GetbBeganPlay))
    (Variables|DONOTEDIT|SetbBeganPlay true)
    (Variables|DONOTEDIT|SetRotationalZ (.yaw (Transformation|GetActorRotation)))
    (Actor|SetLifeSpan (Variables|Gameplay|GetDespawnTime))
    (if (and (Variables|Gameplay|GetbNeedFloor) (not (Variables|DONOTEDIT|GetbDecaying)))
      (CallFunction|CheckforSupportingActors))))

(event EventTick
  (params (DeltaSeconds :type Float%20%28single-precision%29))
  (Networking|SwitchHasAuthority
    (:Authority
      (if (and (Variables|Gameplay|GetbNeedFloor) (not (Variables|DONOTEDIT|GetbDecaying)))
        (CallFunction|CheckforSupportingActors)))))

(event EventUsed
  (params (Invoker :type Actor%20Object%20Reference))
  (Development|PrintString (Utilities|String|Append "I was interacted with by " (Utilities|GetDisplayName Invoker))))

(event Game|Damage|EventPointDamage
  (params (Damage :type Float%20%28single-precision%29) (DamageType :type Damage%20Type%20Object%20Reference) (HitLocation :type Vector :default "0, 0, 0") (HitNormal :type Vector :default "0, 0, 0") (HitComponent :type Primitive%20Component%20Object%20Reference) (BoneName :type Name :default "None") (ShotFromDirection :type Vector :default "0, 0, 0") (InstigatedBy :type Controller%20Object%20Reference) (DamageCauser :type Actor%20Object%20Reference) (HitInfo :type Hit%20Result%20Structure%20%28by%20ref%29))
  (CallFunction|FuncUpdateHealth (* Damage (Variables|Gameplay|GetPointDamageMultiplier)) -1 255))

(event Game|Damage|EventRadialDamage
  (params (DamageReceived :type Float%20%28single-precision%29) (DamageType :type Damage%20Type%20Object%20Reference) (Origin :type Vector :default "0, 0, 0") (HitInfo :type Hit%20Result%20Structure%20%28by%20ref%29) (InstigatedBy :type Controller%20Object%20Reference) (DamageCauser :type Actor%20Object%20Reference))
  (CallFunction|FuncUpdateHealth (* DamageReceived (Variables|Gameplay|GetRadial%20DamageMultiplier)) -1 255))

(fn ConstructionScript
  (Components|StaticMesh|SetStaticMesh (Variables|Default|GetStaticMesh) (Utilities|Array|Get(acopy) (Variables|BuildStages|GetBuildStages))))

(fn OnRepHealth
  (bind _health (Variables|Gameplay|GetHealth))
  (CallFunction|HandleHealthChangeBuildLevel (Variables|DONOTEDIT|GetOldHealth) _health (Variables|DONOTEDIT|GetBuildMode))
  (Variables|DONOTEDIT|SetOldHealth _health))

(fn HandleHealthChangeBuildLevel
  (params (Old%20Health :type Float%20%28single-precision%29) (New%20Health :type Float%20%28single-precision%29) (Build%20Status :type Integer))
  (if (== Build%20Status 1)
    (Variables|DONOTEDIT|SetbBuilt false)
    ;[1 1 1] Health is going DOWN
    ;;[1 1 1] Continue to subsequent checks or stop at lowest build
    (if (>= (Variables|Gameplay|GetHealth) (* (Variables|Gameplay|GetMaximumHealth) (Utilities|Array|Get(acopy) (Variables|BuildStages|GetBuildPercentages)))) :!label _label
      ;;[1 1 1] Continue to 2/3rds health or stop at 1/3rd health static mesh
      (if (>= (Variables|Gameplay|GetHealth) (* (Variables|Gameplay|GetMaximumHealth) (Utilities|Array|Get(acopy) (Variables|BuildStages|GetBuildPercentages) 4)))
        ;;[1 1 1] Continue to 3/3rds health or stop at 2/3rds health static mesh
        (if (>= (Variables|Gameplay|GetHealth) (* (Variables|Gameplay|GetMaximumHealth) (Utilities|Array|Get(acopy) (Variables|BuildStages|GetBuildPercentages) 5)))
          ;;[1 1 1] Stop at 3/3rds
          (Components|StaticMesh|SetStaticMesh (Variables|Default|GetStaticMesh) (Utilities|Array|Get(acopy) (Variables|BuildStages|GetBuildStages) 3))
          (else
            (Components|StaticMesh|SetStaticMesh (Variables|Default|GetStaticMesh) (Utilities|Array|Get(acopy) (Variables|BuildStages|GetBuildStages) 2))))
        (else
          (Components|StaticMesh|SetStaticMesh (Variables|Default|GetStaticMesh) (Utilities|Array|Get(acopy) (Variables|BuildStages|GetBuildStages) 1))))
      (elif (<= (Variables|Gameplay|GetHealth) 0.0)
        (CallFunction|HandleDestroy)
        (else
          (Components|StaticMesh|SetStaticMesh (Variables|Default|GetStaticMesh) (Utilities|Array|Get(acopy) (Variables|BuildStages|GetBuildStages))))))
    (elif (or (< Old%20Health New%20Health) (not (Variables|DONOTEDIT|GetbBuilt)))
      ;[1 1 1] Health is going UP
      ;;[1 1 1] Continue to subsequent checks or stop at lowest build
      (if (>= (Variables|Gameplay|GetHealth) (* (Variables|Gameplay|GetMaximumHealth) (Utilities|Array|Get(acopy) (Variables|BuildStages|GetBuildPercentages))))
        ;;[1 1 1] Continue to 2/3rds health or stop at 1/3rd health static mesh
        (if (>= (Variables|Gameplay|GetHealth) (* (Variables|Gameplay|GetMaximumHealth) (Utilities|Array|Get(acopy) (Variables|BuildStages|GetBuildPercentages) 1)))
          ;;[1 1 1] Continue to 3/3rds health or stop at 2/3rds health static mesh
          (if (>= (Variables|Gameplay|GetHealth) (* (Variables|Gameplay|GetMaximumHealth) (Utilities|Array|Get(acopy) (Variables|BuildStages|GetBuildPercentages) 2)))
            ;;[1 1 1] Stop at 3/3rds
            (Components|StaticMesh|SetStaticMesh (Variables|Default|GetStaticMesh) (Utilities|Array|Get(acopy) (Variables|BuildStages|GetBuildStages) 3))
            (Variables|DONOTEDIT|SetbBuilt true)
            (else
              (Components|StaticMesh|SetStaticMesh (Variables|Default|GetStaticMesh) (Utilities|Array|Get(acopy) (Variables|BuildStages|GetBuildStages) 2))))
          (else
            (Components|StaticMesh|SetStaticMesh (Variables|Default|GetStaticMesh) (Utilities|Array|Get(acopy) (Variables|BuildStages|GetBuildStages) 1))))
        (elif (<= (Variables|Gameplay|GetHealth) 0.0)
          (CallFunction|HandleDestroy)
          (else
            (Components|StaticMesh|SetStaticMesh (Variables|Default|GetStaticMesh) (Utilities|Array|Get(acopy) (Variables|BuildStages|GetBuildStages))))))
      (else
        (goto _label)))))

(fn OnRepRotationalZ
  (Transformation|SetActorRotation (Math|Rotator|MakeRotator 0.0 0.0 (Variables|DONOTEDIT|GetRotationalZ))))

(fn OnRepBuilt
  (CallFunction|HandleRepBuilt))

(fn FuncUpdateHealth
  (params (Change :type Float%20%28single-precision%29) (Build%20Mode :type Integer) (Team :type Byte))
  (bind _damagemultiplier (Variables|Gameplay|GetDamageMultiplier))
  (bind _returnvalue (* Change _damagemultiplier))
  (bind _output_get (Variables|DONOTEDIT|SetBuildMode Build%20Mode))
  (switch int _output_get
    (:Default
      _)
    (:0
      _)
    (:1
      (if (== (Variables|DONOTEDIT|GetOwningTeam) Team)
        (bind _output_get_2 (Variables|Gameplay|SetHealth (Math|Float|Clamp(Float) (- (Variables|Gameplay|GetHealth) _returnvalue) 0.0 (Variables|Gameplay|GetMaximumHealth))))
        (return _output_get_2)
        (else
          (bind _output_get_3 (Variables|Gameplay|SetHealth (Math|Float|Clamp(Float) (- (Variables|Gameplay|GetHealth) (* (Variables|Gameplay|GetEnemyDigDownMultiplier) _returnvalue)) 0.0 (Variables|Gameplay|GetMaximumHealth))))
          (return _output_get_3)))))
  (bind _output_get_4 (Variables|Gameplay|SetHealth (Math|Float|Clamp(Float) (+ _returnvalue (Variables|Gameplay|GetHealth)) 0.0 (Variables|Gameplay|GetMaximumHealth))))
  (return _output_get_4))

(fn FuncDecayTick
  (Networking|SwitchHasAuthority
    (:Authority
      (CallFunction|FuncUpdateHealth 5e+01 1 (Variables|DONOTEDIT|GetOwningTeam)))))

(fn CheckforSupportingActors
  (bind _array_element (Utilities|Array|ForEachLoopwithBreak (Variables|Gameplay|GetSupportLocations) :!label _label)
    (:LoopBody
      (bind (_outhit _returnvalue) (Class|KismetSystemLibrary|BoxTraceSingleforObjects (+ (Math|Vector|RotateVectorAroundAxis (.location _array_element) (.yaw (Transformation|GetActorRotation)) "0, 0,1.000000") (Transformation|GetActorLocation)) (+ (+ (Math|Vector|RotateVectorAroundAxis (.location _array_element) (.yaw (Transformation|GetActorRotation)) "0, 0,1.000000") (Transformation|GetActorLocation)) (Variables|Gameplay|GetSupportCheckTraceDistance)) (Variables|Gameplay|GetSupportCheckHalfSize) (Transformation|GetActorRotation) (Utilities|Array|MakeArray "ObjectTypeQuery1" "ObjectTypeQuery6") false 0 "ForDuration" true "(R=1.000000,G=0.000000,B=0.000000,A=1.000000)" "(R=0.000000,G=1.000000,B=0.000000,A=1.000000)" 1.4))
      (Development|PrintString (Utilities|String|Append (Utilities|GetObjectName self) " supported by " (Utilities|GetObjectName (.hitactor _outhit))) true true "(R=0.000000,G=0.660000,B=1.000000,A=1.000000)" 1.4)
      (bind _output_get (LocalVariables|SetFound _returnvalue))
      (if _output_get
        (goto _label Break)))
    (:Completed
      (Variables|DONOTEDIT|SetbIsSupported (LocalVariables|GetFound)))))

(fn OnRepBIsSupported
  (if (not (Variables|DONOTEDIT|GetbIsSupported))
    (CallFunction|EventBeginDecay false)))