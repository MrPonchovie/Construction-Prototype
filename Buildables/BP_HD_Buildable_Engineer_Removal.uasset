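; BP_HD_Buildable_Engineer_Removal is a buildable that clears its owner's other buildables when spawned.
; On BeginPlay it finds all BP_HD_Buildable_World_Base actors and gives a 0.1-second lifespan to those sharing its owner.
; Actors tagged DSFP_Explosive_Buildable are spared.
; It then sets the same short lifespan on itself, so it acts as a one-shot removal action.
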(event EventBeginPlay
  (|CallParentFunction)
  (bind _outactors (Actor|GetAllActorsOfClass "/HDAssets/Items/Equipment/Utility/Construction/BP_HD_Buildable_World_Base.BP_HD_Buildable_World_Base_C"))
  (for _array_element _outactors
    (if (and (== (Components|GetOwner _array_element) (Components|GetOwner)) (not (Actor|ActorHasTag _array_element "DSFP_Explosive_Buildable")))
      (Actor|SetLifeSpan _array_element 0.1)))
  (Actor|SetLifeSpan 0.1))

(fn ConstructionScript
  (|CallParentFunction))