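; Base world actor for a squad rally point, which enemy players destroy by overrunning it.
; On ownership setup it expires other rallies of the same squad and adds a POI component.
; An opposing-team character entering the radius-configurable overrun sphere triggers destruction, which notifies the owning player's HUD.
; Spawn-point query overrides are stubs returning false, empty or undefined values.
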(event OnComponentBeginOverlap(OverrunSphere)
  (params (OverlappedComponent :type Primitive%20Component%20Object%20Reference) (OtherActor :type Actor%20Object%20Reference) (OtherComp :type Primitive%20Component%20Object%20Reference) (OtherBodyIndex :type Integer) (bFromSweep :type Boolean) (SweepResult :type Hit%20Result%20Structure%20%28by%20ref%29))
  (bind _owningteam (Variables|Default|GetOwningTeam))
  ;[1 1 1] Rally burning
  (bind _ashdplayer_character (Utilities|Casting|CastToHDPlayerCharacter OtherActor))
  (if (not (Math|Boolean|ORBoolean (== (Variables|/Script/DonkehFramework.DFBaseCharacter|GetTeamNum _ashdplayer_character) _owningteam) (== (Variables|Default|GetOwningTeam) 255) (== (Variables|/Script/DonkehFramework.DFBaseCharacter|GetTeamNum _ashdplayer_character) 255)))
    (Development|PrintString (Utilities|String|Append (Utilities|String|ToString(Byte) (Variables|/Script/DonkehFramework.DFBaseCharacter|GetTeamNum _ashdplayer_character)) "   " (Utilities|String|ToString(Byte) _owningteam)))
    (CallFunction|HandleDestroy)))

(event EventEventSetupOwnership
  (params (Owning%20Team :type Byte :default 0) (Owning%20Squad :type HD%20Squad%20State%20Object%20Reference))
  (|CallParentFunction Owning%20Team Owning%20Squad)
  (bind _outactors (Actor|GetAllActorsOfClass "BP_HD_Rally_World_Base_C"))
  (if (> (Utilities|Array|Length _outactors) 0)
    (for _array_element _outactors
      (if (not (== _array_element self))
        (if (== (Variables|/HDAssets/Items/Equipment/Utility/Construction/BP_HD_Buildable_World_Base.BP_HD_Buildable_World_Base_C|GetOwningSquad _array_element) (Variables|Default|GetOwningSquad))
          (Actor|SetLifeSpan _array_element 0.1))))
    ;[1 1 1] Register, Set Up POI
    (bind _returnvalue (AddComponent|AddDFPOIComponent))
    (Variables|Default|SetPOI _returnvalue)))

(event EventHandleDestroy
  (|CallParentFunction)
  (bind _ashdplayer_controller (Utilities|Casting|CastToHDPlayerController (Components|GetOwner)))
  (bind _ashdhud (Utilities|Casting|CastToHDHUD (HUD|GetHUD _ashdplayer_controller))
    (:then
      (bind _asbp_hdhudbase (Utilities|Casting|CastToBP_HDHUDBase _ashdhud)
        (:then
          (Variables|DONOTEDIT|SetNotification%20Widget _asbp_hdhudbase)
          (Default|AddBasicNotification (Variables|DONOTEDIT|GetNotification%20Widget) (Utilities|Struct|MakeFUINotificationInfo false 0 "NewEnumerator0" true "<Normal>Your squad's rally point has been destroyed!</>" "<Normal>{timer}</>" 5.0)))
        (:CastFailed
          (Development|PrintString "Failed BP Cast for HUD" true true "(R=1.000000,G=0.000000,B=0.101476,A=1.000000)"))))
    (:CastFailed
      (Development|PrintString "Failed C++ Cast for Hud" true true "(R=1.000000,G=0.000000,B=0.000000,A=1.000000)"))))

(fn ConstructionScript
  (|CallParentFunction)
  (Components|Sphere|SetSphereRadius (Variables|Default|GetOverrunSphere) (Variables|RallyPoint|GetOverrunRadiusCM) true))

(fn CanRestartPlayerfromSpawnPointBP
  (params (SpawnPoint :type Spawn%20Point%20Def%20Structure%20%28by%20ref%29) (Player :type Controller%20Object%20Reference) (PlayerPawnClass :type Pawn%20Class%20Reference))
  (return false))

(fn CanSpawnActorfromSpawnPointBP
  (params (SpawnPoint :type Spawn%20Point%20Def%20Structure%20%28by%20ref%29) (SpawnActorClass :type Actor%20Class%20Reference))
  (return false))

(fn FindSpawnPointBP
  (params (SpawnPointID :type Integer))
  (return "" false))

(fn GetAllSpawnPointsBP
  (return 0 0))

(fn GetSpawnPointCollisionHandlingOverrideBP
  (params (SpawnPoint :type Spawn%20Point%20Def%20Structure%20%28by%20ref%29))
  (return "Undefined" false))